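; Gluttony enemy character that roams, patrols or chases the player, starting from its EAISTATE value.
; Patrol walks a loop of four target points with pauses, while Roam repeatedly picks random nearby navigable points.
; Pawn sensing starts a flying chase that destroys the player on a successful move and returns to patrol after delays.
; While the player is flagged as seen, Tick re-issues Chase, or Patrol if the player is hiding.
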(event OnSeePawn(PawnSensing)
  (params (Pawn :type Pawn%20Object%20Reference))
  (bind _ascharacter_sinful (Utilities|Casting|CastToCharacter_Sinful Pawn))
  (Default|StartBeingChased _ascharacter_sinful)
  (CallFunction|Chase)
  (Default|StopBeingChased _ascharacter_sinful))

(event Custom|Roam
  (AI|AIMoveTo self (.RandomLocation (Class|NavigationSystem|GetRandomPointinNavigableRadius (Transformation|GetActorLocation) 5e+02)) 0 5.0 false
    (:then
      (Utilities|FlowControl|Delay 1.0)
      (CallFunction|Roam))))

(event Custom|Chase
  (bind _returnvalue (Game|GetPlayerCharacter 0))
  (Pawn|Components|CharacterMovement|SetMovementMode (Variables|Character|GetCharacterMovement) "MOVE_Flying" 0)
  (Variables|Default|SetSawPlayer true)
  (AI|AIMoveTo self "0, 0, 0" _returnvalue 1e+01 true
    (:then
      (Utilities|FlowControl|Delay 1e+01)
      (Variables|Default|SetSawPlayer false)
      (Utilities|FlowControl|Delay 1e+01))
    (:OnSuccess
      (Utilities|FlowControl|Delay 0.2)
      (Actor|DestroyActor _returnvalue)
      (Variables|Default|SetSawPlayer false)))
  (CallFunction|Patrol))

(event Custom|Patrol
  (Pawn|Components|CharacterMovement|SetMovementMode (Variables|Character|GetCharacterMovement) "MOVE_Walking" 0)
  (AI|AIMoveTo self "0, 0, 0" (Variables|Default|GetTargetPoint1) 5.0 false
    (:OnSuccess
      (Utilities|FlowControl|Delay 2.5)
      (AI|AIMoveTo self "0, 0, 0" (Variables|Default|GetTargetPoint2) 5.0 false
        (:OnSuccess
          (Utilities|FlowControl|Delay 2.5)
          (AI|AIMoveTo self "0, 0, 0" (Variables|Default|GetTargetPoint3) 5.0 false
            (:OnSuccess
              (Utilities|FlowControl|Delay 2.5)
              (AI|AIMoveTo self "0, 0, 0" (Variables|Default|GetTargetPoint4) 5.0 false
                (:OnSuccess
                  (CallFunction|Patrol))))))))))

(event EventBeginPlay
  (switch Utilities|FlowControl|Switch|Switchon (Variables|Default|GetEAISTATE)
    (:NewEnumerator1
      (CallFunction|Roam))
    (:NewEnumerator2
      (CallFunction|Chase))
    (:NewEnumerator3
      (CallFunction|Patrol))))

(event EventTick
  (params (DeltaSeconds :type Float%20%28single-precision%29))
  (if (Variables|Default|GetSawPlayer)
    (bind _ascharacter_sinful (Utilities|Casting|CastToCharacter_Sinful (Game|GetPlayerCharacter 0)))
    (if (Variables|/Game/Blueprints/Character_Sinful.Character_Sinful_C|GetbIsHiding _ascharacter_sinful)
      (CallFunction|Patrol)
      (else
        (CallFunction|Chase)))))

(fn ConstructionScript)