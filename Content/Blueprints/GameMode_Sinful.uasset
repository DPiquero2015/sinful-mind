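; GameMode_Sinful is a game mode Blueprint that respawns the player's Character_Sinful whenever it is destroyed.
; On BeginPlay it binds the Destroyed event to the player character's OnDestroyed.
; After a short delay, that event spawns a new Character_Sinful at the stored SpawnTransform, has the player controller possess it, and calls Respawn to rebind the event.
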(event Custom|Destroyed
  (params (DestroyedActor :type Actor%20Object%20Reference))
  (Utilities|FlowControl|Delay 0.2)
  (bind _returnvalue (Game|SpawnActorfromClass "/Game/Blueprints/Character_Sinful.Character_Sinful_C" (Variables|Default|GetSpawnTransform) "Undefined" 0 0))
  (Pawn|Possess (Game|GetPlayerController 0) _returnvalue)
  (CallFunction|Respawn))

(event Custom|Respawn
  (Utilities|Casting|CastToCharacter_Sinful (Game|GetPlayerCharacter 0))
  (EventDispatchers|BindEventtoOnDestroyed (delegate Custom|Destroyed)))

(event EventBeginPlay
  (Utilities|Casting|CastToCharacter_Sinful (Game|GetPlayerCharacter 0))
  (EventDispatchers|BindEventtoOnDestroyed (delegate Custom|Destroyed)))

(event EventTick
  (params (DeltaSeconds :type Float%20%28single-precision%29)))

(fn ConstructionScript)