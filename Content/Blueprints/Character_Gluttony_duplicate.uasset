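; Enemy AI character that roams, patrols or chases the player, and self-destructs with an explosion effect and sound on reaching them.
; AIState selects the starting behavior: repeated random navmesh moves, a four-target-point patrol loop, or a chase.
; Pawn sensing triggers Chase, which Tick re-issues while SawPlayer is set.
; Delays after the chase starts clear that flag, then return the character to patrol.
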(event OnSeePawn(PawnSensing)
  (params (Pawn :type Pawn%20Object%20Reference))
  (Utilities|Casting|CastTo Pawn)
  (CallFunction|Chase))

(event Custom|Roam
  (AI|AIMoveTo self (.RandomLocation (Class|NavigationSystem|GetRandomPointinNavigableRadius (Transformation|GetActorLocation) 5e+02)) 0 5.0 false
    (:then
      (Utilities|FlowControl|Delay 1.0)
      (CallFunction|Roam))))

(event Custom|Chase
  (bind _returnvalue (Transformation|GetActorLocation))
  (Variables|Default|SetSawPlayer true)
  (AI|AIMoveTo self "0, 0, 0" (Game|GetPlayerCharacter 0) 5.0 false
    (:then
      (Utilities|FlowControl|Delay 1e+01)
      (Variables|Default|SetSawPlayer false)
      (Utilities|FlowControl|Delay 1e+01)
      (CallFunction|Patrol))
    (:OnSuccess
      (Effects|SpawnEmitteratLocation "/Game/StarterContent/Particles/P_Explosion.P_Explosion" _returnvalue)
      (Audio|PlaySoundatLocation "/Game/StarterContent/Audio/Explosion_Cue.Explosion_Cue" _returnvalue)
      (Actor|DestroyActor))))

(event Custom|Patrol
  (AI|AIMoveTo self "0, 0, 0" (Variables|Default|GetTargetPoint1) 5.0 false
    (:OnSuccess
      (Utilities|FlowControl|Delay 2.5)
      (AI|AIMoveTo self "0, 0, 0" (Variables|Default|GetTargetPoint2) 5.0 false
        (:OnSuccess
          (Utilities|FlowControl|Delay 2.5)
          (AI|AIMoveTo self "0, 0, 0" (Variables|Default|GetTargetPoint3) 5.0 false
            (:OnSuccess
              (Utilities|FlowControl|Delay 2.5)
              (AI|AIMoveTo self "0, 0, 0" (Variables|Default|GetTargetPoint4) 5.0 false
                (:OnSuccess
                  (CallFunction|Patrol))))))))))

(event EventBeginPlay
  (switch Utilities|FlowControl|Switch|Switchon (Variables|Default|GetAIState)
    (:NewEnumerator1
      (CallFunction|Roam))
    (:NewEnumerator2
      (CallFunction|Chase))
    (:NewEnumerator3
      (CallFunction|Patrol))))

(event EventTick
  (params (DeltaSeconds :type Float%20%28single-precision%29))
  (if (Variables|Default|GetSawPlayer)
    (CallFunction|Chase)))

(fn ConstructionScript)