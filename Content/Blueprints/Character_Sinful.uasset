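; First-person style player character that moves, jumps, uses interactables and can hide in spots.
; A per-tick camera line trace finds nearby I_Interactable actors for the Interact input, which instead exits hiding when hidden.
; Hide and UnHide use a timeline to blend actor transform and control rotation, toggling Flying and Falling modes.
; While hidden, movement and jump input are ignored and look is clamped around the hiding spot's facing.
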(event Custom|Check%20For%20Interactables
  (bind _camera (Variables|Default|GetCamera))
  (bind _returnvalue (Transformation|GetWorldLocation _camera))
  (bind (_outhit _returnvalue_2) (Collision|LineTraceByChannel _returnvalue (+ _returnvalue (* (Math|Vector|GetForwardVector _camera) 200)) "TraceTypeQuery2" false 0 "ForOneFrame"))
  (if _returnvalue_2
    (if (Utilities|DoesObjectImplementInterface (.HitActor (Collision|BreakHitResult _outhit)) "/Game/Blueprints/I_Interactable.I_Interactable_C")
      (Variables|Default|SetInteractable (.HitActor (Collision|BreakHitResult _outhit)))
      (Variables|Default|SetbCanInteract true))
    (else
      (Variables|Default|SetbCanInteract false))))

(event Custom|UnHide
  (CallFunction|LerpTransform (Transformation|GetActorTransform) (Variables|Default|GetPlaced) (Pawn|GetControlRotation :!class /Script/Engine.Pawn))
  (Pawn|Components|CharacterMovement|SetMovementMode (Variables|Character|GetCharacterMovement) "MOVE_Falling" 0)
  (Variables|Default|SetbIsHiding false))

(event Custom|Hide
  (Variables|Default|SetbIsHiding true)
  (CallFunction|LerpTransform (Transformation|GetActorTransform) (Variables|Default|GetHiding) (Pawn|GetControlRotation :!class /Script/Engine.Pawn))
  (CallFunction|StopMoving))

(event Custom|Lerp%20Transform
  (params (Start :type Transform) (End :type Transform) (Camera :type Rotator))
  (bind _alpha (Timeline|Lerp PlayFromStart)
    (:Update
      (Transformation|SetActorTransform (Math|Transform|Lerp(Transform) Start End _alpha))
      (Pawn|SetControlRotation (Pawn|GetController) (Math|Rotator|Lerp(Rotator) Camera (.Rotation (Math|Transform|BreakTransform End)) _alpha true)))))

(event Custom|Stop%20Moving
  (bind _charactermovement (Variables|Character|GetCharacterMovement))
  (Pawn|Components|CharacterMovement|SetMovementMode _charactermovement "MOVE_Flying" 0)
  (Components|Movement|StopMovementImmediately _charactermovement))

(event EventTick
  (params (DeltaSeconds :type Float%20%28single-precision%29))
  (CallFunction|CheckforInteractables))

(event Input|ActionEvents|InputActionJump
  (params (Key :type Key%20Structure))
  (bind _bishiding (Variables|Default|GetbIsHiding))
  (:Pressed
    (if (not _bishiding)
      (Character|Jump)))
  (:Released
    (if (not _bishiding)
      (Character|StopJumping))))

(event Input|ActionEvents|InputActionInteract
  (params (Key :type Key%20Structure))
  (:Pressed
    (if (Variables|Default|GetbIsHiding)
      (CallFunction|UnHide)
      (elif (Variables|Default|GetbCanInteract)
        (Class|IInteractable|IInteract(Message) (Variables|Default|GetInteractable))))))

(event Input|AxisEvents|InputAxisDolly
  (params (AxisValue :type Float%20%28single-precision%29))
  (if (not (Variables|Default|GetbIsHiding))
    (Pawn|Input|AddMovementInput (Transformation|GetActorForwardVector) AxisValue false)))

(event Input|AxisEvents|InputAxisTruck
  (params (AxisValue :type Float%20%28single-precision%29))
  (if (not (Variables|Default|GetbIsHiding))
    (Pawn|Input|AddMovementInput (Transformation|GetActorRightVector) AxisValue false)))

(event Input|AxisEvents|InputAxisPan
  (params (AxisValue :type Float%20%28single-precision%29))
  (Pawn|Input|AddControllerYawInput AxisValue)
  (if (Variables|Default|GetbIsHiding)
    (CallFunction|RestrictCamera)))

(event Input|AxisEvents|InputAxisTilt
  (params (AxisValue :type Float%20%28single-precision%29))
  (Pawn|Input|AddControllerPitchInput AxisValue)
  (if (Variables|Default|GetbIsHiding)
    (CallFunction|RestrictCamera)))

(fn ConstructionScript)

(fn RestrictCamera
  (bind _returnvalue (Pawn|GetControlRotation :!class /Script/Engine.Pawn))
  (bind _hiding (Variables|Default|GetHiding))
  (Pawn|SetControlRotation (Pawn|GetController) (Math|Rotator|MakeRotator (.roll _returnvalue) (Math|Float|ClampAngle (.pitch _returnvalue) -45.0 45.0) (Math|Float|ClampAngle (.yaw _returnvalue) (- (.yaw (.rotation _hiding)) 45.0) (+ (.yaw (.rotation _hiding)) 45.0)))))